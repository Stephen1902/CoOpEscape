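; BP_InteractiveCollection is an interactive world item that leaves its overlap and interact behavior to its parent class.
; Its overlap begin, overlap end and interact handlers only forward to the parent implementations.
; GetName prints debug strings and returns the item's Name with the DT_InteractiveInfo data table.
; Outline highlighting, inventory pickup and IsPlaced visibility logic remain as disconnected nodes, leaving OnRep_IsPlaced empty.
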(event `self.ReceiveBeginPlay`)

(event `InteractInterface.OnOverlapEnd`
  (`parent.OnOverlapEnd`))

(event `InteractInterface.OnInteractBegin`
  (`parent.OnInteractBegin`))

(fn `GetName`
  (returns (DataTableOut :type "DataTable Object Reference") (ReturnValue :type Name))
  (bind _name (`self.Name`))
  (`KismetSystemLibrary.PrintString` "Get Name Called BP")
  (`KismetSystemLibrary.PrintString` (`KismetStringLibrary.Conv_NameToString` _name))
  (return "/Game/Framework/DT_InteractiveInfo.DT_InteractiveInfo" _name))

(fn `OnOverlapBegin`
  (params (OwnerIn :type "Actor Object Reference"))
  (returns (ReturnValue :type "Actor Object Reference"))
  (bind _returnvalue (`parent.OnOverlapBegin` OwnerIn))
  (return _returnvalue))

(fn `OnRep_IsPlaced`)

(fn `UserConstructionScript`)