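; Weighing scale world item that shows the weight of items resting on it and reports activation when that matches a target weight.
; Every Tick it sums weights from Box-overlapping actors implementing InteractInterface, then compares with TargetWeight within a small tolerance whenever the total changes.
; Weight display goes through WeightText, whose RepNotify sets the TextRender.
; Emptying the box resets the total and text without signalling an activation change.
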(event `self.ReceiveTick`
  (params (DeltaSeconds :type "Float (single-precision)"))
  (bind _overlappingactors (`PrimitiveComponent.GetOverlappingActors` (`self.Box`) null))
  (if (> (`KismetArrayLibrary.Array_Length` _overlappingactors) 0)
    (set `self.RunningWeight` 0.0)
    (for _array_element _overlappingactors
      (if (`KismetSystemLibrary.DoesImplementInterface` _array_element "/Script/CoOpEscape.InteractInterface")
        (bind _returnvalue (message `InteractInterface.GetItemWeight` _array_element))
        (set `self.RunningWeight` (+ _returnvalue (`self.RunningWeight`)))))
    (if (!= (`self.CurrentWeight`) (`self.RunningWeight`))
      (set `self.CurrentWeight` (`self.RunningWeight`))
      (`self.UpdateTextInfo`)
      (if (`KismetMathLibrary.NearlyEqual_FloatFloat` (`self.CurrentWeight`) (`self.TargetWeight`) 0.001)
        (`self.OnActivatedChange` true)
        (else
          (`self.OnActivatedChange` false))))
    (elif (> (`self.CurrentWeight`) 0.0)
      (set `self.CurrentWeight` 0.0)
      (`self.UpdateTextInfo`))))

(event `UpdateTextInfo`
  (set `self.WeightText` (`KismetTextLibrary.Conv_DoubleToText` (`self.CurrentWeight`) "HalfToEven")))

(event `Server_UpdateTextInfo`
  (`self.UpdateTextInfo`))

(fn `OnRep_WeightText`
  (`TextRenderComponent.K2_SetText` (`self.TextRender`) (`self.WeightText`)))

(fn `UserConstructionScript`)