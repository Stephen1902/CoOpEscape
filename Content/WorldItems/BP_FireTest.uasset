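; BP_FireTest is a test world-item actor that burns up when triggered and then destroys itself.
; Triggering activates its particle system and creates a dynamic material instance on the mesh.
; A timeline scales the material's SurfaceColor by its float value, then destroys the actor when finished.
; Untriggering only deactivates the particles, leaving any running timeline to complete.
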(event `self.OnIsTriggeredTrue`
  (`self.DisplayChanges` true))

(event `DisplayChanges`
  (params (IsActive :type Boolean))
  (bind _meshcomp (`self.MeshComp`))
  (if IsActive
    (`ActorComponent.Activate` (`self.ParticleSystem`) false)
    (bind _returnvalue (`PrimitiveComponent.CreateDynamicMaterialInstance` _meshcomp 0 (`PrimitiveComponent.GetMaterial` _meshcomp 0) "None"))
    (`PrimitiveComponent.SetMaterial` (`self.MeshComp`) 0 _returnvalue)
    (bind _returnvalue_2 (`MaterialInstanceDynamic.K2_GetVectorParameterValue` _returnvalue "SurfaceColor"))
    (bind (_direction _float_value) (`Timeline|Timeline`)
      (:`Update`
        (`MaterialInstanceDynamic.SetVectorParameterValue` _returnvalue "SurfaceColor" (* _returnvalue_2 _float_value)))
      (:`Finished`
        (`self.K2_DestroyActor`)))
    (else
      (`ActorComponent.Deactivate` (`self.ParticleSystem`)))))

(event `self.OnIsTriggeredFalse`
  (`self.DisplayChanges` false))

(fn `UserConstructionScript`)