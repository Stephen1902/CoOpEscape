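; BP_InteractiveTest is a test world item that shows interaction state by swapping the material on its mesh.
; BeginPlay caches the original material; overlap begin applies a floor material and returns self, overlap end restores the original, and interaction applies clay brick.
; All changes go through MCUpdateMaterial, apparently a multicast, with interaction branching on authority to call it directly or via a server event.
; Owner assignment in OnOverlapBegin is disconnected.
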(event `self.ReceiveBeginPlay`
  (set `self.DefaultMaterial` (`PrimitiveComponent.GetMaterial` (`self.MeshComp`) 0)))

(event `InteractInterface.OnOverlapEnd`
  (`self.MC Update Material` (`self.DefaultMaterial`)))

(event `MC Update Material`
  (params (Material :type "MaterialInterface Object Reference"))
  (`PrimitiveComponent.SetMaterial` (`self.MeshComp`) 0 Material))

(event `InteractInterface.OnInteractBegin`
  (`/Engine/EditorBlueprintResources/ActorMacros.Switch Has Authority`
    (:`Authority`
      (`self.MC Update Material` "/Game/StarterContent/Materials/M_Brick_Clay_New.M_Brick_Clay_New"))
    (:`Remote`
      (`self.Server_UpdateMaterial`))))

(event `Server_UpdateMaterial`
  (`self.MC Update Material` "/Game/StarterContent/Materials/M_Brick_Clay_New.M_Brick_Clay_New"))

(fn `OnOverlapBegin`
  (params (OwnerIn :type "Actor Object Reference"))
  (returns (ReturnValue :type "Actor Object Reference"))
  (`self.MC Update Material` "/Game/StarterContent/Materials/M_Basic_Floor.M_Basic_Floor")
  (return self))

(fn `UserConstructionScript`)